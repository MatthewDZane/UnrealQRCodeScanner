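; OpenCV scene capture actor Blueprint that sizes a display plane to match the aspect ratio of its capture render target.
; BeginPlay runs the parent logic, then starts a one-shot delayed timer that calls SetResolution.
; SetResolution scales the Plane in world space from the texture target's width-to-height ratio and PlaneHeight.
; Any capture or OpenCV processing lives outside this graph, as Tick only calls its parent.
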(event Custom|SetResolution
  (bind _plane_height (Variables|Default|GetPlane%20Height))
  (bind _scenecapturecomponent (Variables|Default|GetsceneCaptureComponent))
  (bind _texturetarget (Variables|/Script/Engine.SceneCaptureComponent2D|GetTextureTarget _scenecapturecomponent))
  ;[1 1 1] Set Plane to the same scale as the Texture Target Resolution
  (Transformation|SetWorldScale3D (Variables|Default|GetPlane) (Math|Vector|MakeVector (* (/ (Math|Conversions|ToFloat(Integer) (Variables|/Script/Engine.TextureRenderTarget2D|GetSizeX _texturetarget)) (Math|Conversions|ToFloat(Integer) (Variables|/Script/Engine.TextureRenderTarget2D|GetSizeY _texturetarget))) _plane_height) _plane_height _plane_height)))

(event EventBeginPlay
  (|CallParentFunction)
  (Utilities|Time|SetTimerbyEvent (delegate Custom|SetResolution) 5.0))

(event Collision|EventActorBeginOverlap
  (params (OtherActor :type Actor%20Object%20Reference)))

(event EventTick
  (params (DeltaSeconds :type Float%20%28single-precision%29))
  (|CallParentFunction DeltaSeconds))

(fn ConstructionScript)