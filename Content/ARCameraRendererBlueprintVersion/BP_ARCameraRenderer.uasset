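; BP_ARCameraRenderer is an actor that shows the AR camera image on a plane.
; BeginPlay starts an AR session with camera capture, and EndPlay shuts both down.
; After a short delay it gives the plane a dynamic material, then uses a timer meant to retry until the camera texture is valid.
; It then binds the texture once and sets plane scale from the camera resolution's aspect ratio.
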(event Custom|OnMaterialTimer
  ;[1 1 1] Update Plane Texture with Camera Image
  (bind _returnvalue (Class|ARBlueprintLibrary|GetARTexture "CameraImage"))
  (Utilities|IsValid _returnvalue
    (:Is%20Valid
      (Rendering|Material|SetTextureParameterValue (stale Custom|OnTimerDelay _returnvalue) "Param" _returnvalue)
      ;[1 1 1] Get Camera Intrinsics and Scale Preview Plane to Resolution of Camera
      (bind _outcameraintrinsics (Class|ARBlueprintLibrary|GetCameraIntrinsics))
      (Transformation|SetWorldScale3D (Variables|Default|GetPlane) (Math|Vector|MakeVector (/ (Math|Conversions|ToFloat(Integer) (.X (Utilities|Struct|BreakIntPoint (.ImageResolution (Utilities|Struct|BreakARCameraIntrinsics _outcameraintrinsics))))) (Math|Conversions|ToFloat(Integer) (.Y (Utilities|Struct|BreakIntPoint (.ImageResolution (Utilities|Struct|BreakARCameraIntrinsics _outcameraintrinsics)))))) 0.0 0.0)))
    (:Is%20Not%20Valid
      (Utilities|Time|SetTimerbyEvent (delegate Custom|OnMaterialTimer) 0.0))))

(event Custom|OnTimerDelay
  (bind _returnvalue (Rendering|Material|CreateDynamicMaterialInstance "/UnrealQRCodeScanner/ARCameraRendererBlueprintVersion/M_ARCameraTexture.M_ARCameraTexture" "None" "None" :!class /Script/Engine.KismetMaterialLibrary))
  (Rendering|Material|SetMaterial (Variables|Default|GetPlane) 0 _returnvalue)
  (Utilities|Time|SetTimerbyEvent (delegate Custom|OnMaterialTimer) 0.0))

(event EventBeginPlay
  (Class|ARBlueprintLibrary|StartARSession "/UnrealQRCodeScanner/DA_ARSessionConfig.DA_ARSessionConfig")
  (Class|ARBlueprintLibrary|ToggleARCapture true "Camera")
  (Utilities|Time|SetTimerbyEvent (delegate Custom|OnTimerDelay) 0.1))

(event EventEndPlay
  (params (EndPlayReason :type EEndPlayReason%20Enum :default "Destroyed"))
  ;[1 1 1] Disable Camera Capture and End Session
  (Class|ARBlueprintLibrary|ToggleARCapture false "Camera")
  (Class|ARBlueprintLibrary|StopARSession))

(fn ConstructionScript)