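; BP_OpenCVSceneCapture is a scene capture Blueprint that displays an OpenCV camera texture on a screen mesh.
; A timer after BeginPlay creates a dynamic material on ScreenMesh, then binds CameraTexture2D to it after a short delay.
; It also scales the mesh to the capture target's aspect ratio using PlaneHeight.
; Each Tick draws that material into CameraRenderTarget once both are valid.
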(event Custom|SetResolution
  (bind _scenecapturecomponent (Variables|Default|GetsceneCaptureComponent))
  (bind _plane_height (Variables|Default|GetPlane%20Height))
  (bind _texturetarget (Variables|/Script/Engine.SceneCaptureComponent2D|GetTextureTarget _scenecapturecomponent))
  ;[1 1 1] Create Material for Screen Component
  (bind _returnvalue (Rendering|Material|CreateDynamicMaterialInstance (Variables|Default|GetScreen%20Mesh) 0 "/UnrealQRCodeScanner/OpenCVSceneCapture/M_OpenCVSceneCapture.M_OpenCVSceneCapture" "None" :!class /Script/Engine.PrimitiveComponent))
  (Variables|Default|SetCamera_Mat _returnvalue)
  (Utilities|FlowControl|Delay 0.2)
  (Rendering|Material|SetTextureParameterValue (Variables|Default|GetCamera_Mat) "Param" (Variables|Default|GetCamera_Texture2D))
  ;[1 1 1] Set Plane to the same scale as the Texture Target Resolution
  (Transformation|SetWorldScale3D (Variables|Default|GetScreen%20Mesh) (Math|Vector|MakeVector (* (/ (Math|Conversions|ToFloat(Integer) (Variables|/Script/Engine.TextureRenderTarget2D|GetSizeX _texturetarget)) (Math|Conversions|ToFloat(Integer) (Variables|/Script/Engine.TextureRenderTarget2D|GetSizeY _texturetarget))) _plane_height) _plane_height _plane_height)))

(event EventBeginPlay
  (|CallParentFunction)
  (Utilities|Time|SetTimerbyEvent (delegate Custom|SetResolution) 5.0))

(event EventTick
  (params (DeltaSeconds :type Float%20%28single-precision%29))
  (bind _camera_rendertarget (Variables|Default|GetCamera_RenderTarget))
  (bind _camera_mat (Variables|Default|GetCamera_Mat))
  (|CallParentFunction DeltaSeconds)
  (Utilities|IsValid _camera_rendertarget
    (:Is%20Valid
      (Utilities|IsValid _camera_mat
        (:Is%20Valid
          (Rendering|DrawMaterialtoRenderTarget _camera_rendertarget _camera_mat))))))

(fn ConstructionScript)