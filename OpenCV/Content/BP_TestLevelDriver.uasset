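; Test level driver actor that starts an AR session with OpenXR hand mesh visualization and camera capture, then displays device camera feeds.
; After a delay, which lets capture toggle on before cameras open, it spawns BP_ExternalCameraRenderer, rotated for correct sensor preview, and the C++ ARCameraRenderer for the PV camera.
; EndPlay stops the AR session.
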(event Custom|SpawnCameraObjects
  ;[1 1 1] Camera Capture must be toggled prior to opening cameras on device
  (Game|SpawnActorfromClass "/Game/ExternalCameraReader/BP_ExternalCameraRenderer.BP_ExternalCameraRenderer_C" (Math|Transform|MakeTransform "400.000000, 0,120.000000" "0.000000, 0,90.000000") "Undefined" 0 0)
  ;[1 1 1] Spawn C++ Actor to render pv camera
  (Game|SpawnActorfromClass "/Script/OpenCV.ARCameraRenderer" (Math|Transform|MakeTransform "400.000000,400.000000,200.000000") "Undefined" 0 0))

(event EventBeginPlay
  ;[1 1 1] Start AR and Enable OpenXR HandMesh
  (Class|ARBlueprintLibrary|StartARSession "/Game/DA_ARSessionConfig.DA_ARSessionConfig")
  (Class|MicrosoftOpenXRFunctionLibrary|SetUseHandMesh "EnabledXRVisualization")
  (Class|ARBlueprintLibrary|ToggleARCapture true "Camera")
  ;[1 1 1] Camera Capture must be toggled prior to opening cameras on device
  (Utilities|Time|SetTimerbyEvent (delegate Custom|SpawnCameraObjects) 1e+01))

(event EventEndPlay
  (params (EndPlayReason :type EEndPlayReason%20Enum :default "Destroyed"))
  ;[1 1 1] Stop AR Process
  (Class|ARBlueprintLibrary|StopARSession))

(fn ConstructionScript)