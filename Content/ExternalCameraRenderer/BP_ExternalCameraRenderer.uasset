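; BP_ExternalCameraRenderer is an actor that draws an external camera texture onto a screen mesh and into a render target.
; Five seconds after BeginPlay it creates a dynamic M_ExternalCamera material on ScreenMesh, then assigns CameraTexture2D after a short delay.
; Tick draws that material into CameraRenderTarget every frame when both are valid.
; Logic to open a capture device by CameraID in CameraMediaPlayer exists but never runs.
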(event Custom|StartCapture
  ;[1 1 1] Create Material for Screen Component
  (bind _returnvalue (Rendering|Material|CreateDynamicMaterialInstance (Variables|Default|GetScreen_Mesh) 0 "/UnrealQRCodeScanner/ExternalCameraRenderer/M_ExternalCamera.M_ExternalCamera" "None" :!class /Script/Engine.PrimitiveComponent))
  (Variables|Default|SetCamera_Mat _returnvalue)
  (Utilities|FlowControl|Delay 0.2)
  (Rendering|Material|SetTextureParameterValue (Variables|Default|GetCamera_Mat) "Param" (Variables|Default|GetCamera_Texture2D)))

(event EventBeginPlay
  (|CallParentFunction)
  (Utilities|Time|SetTimerbyEvent (delegate Custom|StartCapture) 5.0))

(event EventTick
  (params (DeltaSeconds :type Float%20%28single-precision%29))
  (bind _camera_mat (Variables|Default|GetCamera_Mat))
  (bind _camera_rendertarget (Variables|Default|GetCamera_RenderTarget))
  (|CallParentFunction DeltaSeconds)
  (Utilities|IsValid _camera_rendertarget
    (:Is%20Valid
      (Utilities|IsValid _camera_mat
        (:Is%20Valid
          (Rendering|DrawMaterialtoRenderTarget _camera_rendertarget _camera_mat))))))

(fn ConstructionScript)